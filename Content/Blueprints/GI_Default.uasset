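; GI_Default is the Game Instance that keeps the session's best score and running point total, both reset on Init.
; UpdateGlobalScore raises BestScore when matched or beaten, then adds scaled points to CurrentPoints, with a 5% bonus if Has5Points is set.
; The event feeds a constant zero into the points formula instead of the incoming score, so awarded points vary only with scale and bonus.
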(event `self.ReceiveInit`
  (set `self.BestScore` 0.0)
  (set `self.CurrentPoints` 0))

(event `UpdateGlobalScore`
  (params (Score :type "Float (double-precision)") (PointScale :type "Float (double-precision)") (`Has5%Points` :type Boolean))
  (`self.UpdateBestScore` Score)
  (`self.UpdatePoints` 0.0 PointScale `Has5%Points`))

(fn `CalculatePointsFromScore`
  (params (Score :type "Float (double-precision)") (Scale :type "Float (double-precision)"))
  (returns (Points :type Integer))
  (return (`KismetMathLibrary.Round` (* (/ (* (+ Score 50.0) 100.0) 2.0) Scale))))

(fn `UpdateBestScore`
  (params (Score :type "Float (double-precision)"))
  (if (>= Score (`self.BestScore`))
    (set `self.BestScore` Score)))

(fn `UpdatePoints`
  (params (Score :type "Float (double-precision)") (Scale :type "Float (double-precision)") (`Has5%Points` :type Boolean))
  (bind _points (`self.CalculatePointsFromScore` Score Scale))
  (set `self.CurrentPoints` (+ _points (`self.CurrentPoints`) (select `bool` `Has5%Points` :`true` (`KismetMathLibrary.Round` (* _points 0.05))))))