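; BP_Enemy is a flying enemy that chases the player and damages whatever it hits.
; Construction pulls mesh, stats and effects from DT_Enemies by EnemyId.
; Once inside ChaseRadius, it permanently homes in each tick, slowing sharply behind the player (dot-product angle test) and despawning if also far away.
; Hits trigger particles, sound and death, except pickup hits unless DieOnPickupHit is set.
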(event `self.ReceiveBeginPlay`
  (`/Engine/EditorBlueprintResources/StandardMacros.IsValid` (`self.PlayerRef`)
    (:`Is Not Valid`
      (bind _returnvalue (`GameplayStatics.GetActorOfClass` "/Game/Blueprints/BP_Player.BP_Player_C"))
      (set `self.PlayerRef` _returnvalue)
      (`SceneComponent.K2_SetWorldRotation` (`self.RootComponent`) (`self.GetLookAtRotToPlayer`) false false))))

(event `self.ReceiveTick`
  (params (DeltaSeconds :type "Float (single-precision)"))
  (bind (_enemydata_enemyid _enemydata_displayname _enemydata_flyspeed _enemydata_damage _enemydata_chaseradius) (break `/Game/Blueprints/BP_EnemyStruct` (`self.EnemyData`)))
  ;[1 1 1] Make sure we are within the aggro radius or if we are already chasing the player
  (if (or (<= (`self.GetDistanceToPlayer`) _enemydata_chaseradius) (`self.IsChasing`))
    (set `self.IsChasing` true)
    ;[1 1 1] Rotate and look at the player
    (`SceneComponent.K2_SetWorldRotation` (`self.RootComponent`) (`self.GetLookAtRotToPlayer`) false false)
    ;[1 1 1] Move towards the player
    (`self.AddMovementInput` (`self.GetDirectionToPlayer`) (`self.GetScaledSpeed` _enemydata_flyspeed))
    (if (and (`self.IsBehindPlayer` 30.0) (>= (`self.GetDistanceToPlayer`) 3000.0))
      (`self.K2_DestroyActor`))))

(event `Die`
  (`self.K2_DestroyActor`))

(event `self.CollisionComponent.OnComponentHit`
  (params (HitComponent :type "PrimitiveComponent Object Reference") (OtherActor :type "Actor Object Reference") (OtherComp :type "PrimitiveComponent Object Reference") (NormalImpulse :type "Vector Structure") (Hit :type "HitResult Structure (by ref)"))
  (bind (_bblockinghit _binitialoverlap _time _distance _location _impactpoint) (`GameplayStatics.BreakHitResult` Hit))
  (bind (_enemydata_enemyid _enemydata_displayname _enemydata_flyspeed _enemydata_damage _enemydata_chaseradius _enemydata_dieonpickuphit _enemydata_staticmesh _enemydata_spawnweight _enemydata_hitparticles _enemydata_hitsfx) (break `/Game/Blueprints/BP_EnemyStruct` (`self.EnemyData`)))
  (`GameplayStatics.ApplyDamage` OtherActor _enemydata_damage null self)
  (cast `/Game/Blueprints/BP_Pickup` OtherActor
    (:`then`
      (if _enemydata_dieonpickuphit
        (`GameplayStatics.SpawnEmitterAtLocation` _enemydata_hitparticles _impactpoint :!label _label)
        (`GameplayStatics.PlaySoundAtLocation` _enemydata_hitsfx _impactpoint (struct) 1.0 1.0 0.0 null null null)
        (`self.Die`)))
    (:`CastFailed`
      (goto _label))))

(fn `UserConstructionScript`
  (bind _returnvalue (`|GetDataTableRow` "/Game/Blueprints/DT_Enemies.DT_Enemies" (`self.EnemyId`))
    (:`then`
      (bind _output_get (set `self.EnemyData` _returnvalue)))
    (:`RowNotFound`
      (set `self.EnemyData` (make `/Game/Blueprints/BP_EnemyStruct` "None" "Unknown" 5.0 1.0 9999999.0 false "/Engine/BasicShapes/Cone.Cone"))))
  (`StaticMeshComponent.SetStaticMesh` (`self.StaticMesh`) (`.StaticMesh_17_B3DA964A4EA863AFFDCD698FB6EC120B` (break `/Game/Blueprints/BP_EnemyStruct` _output_get))))