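; Enemy spawner actor that, when enabled, spawns NumItems BP_Enemy actors on BeginPlay, each with an EnemyId drawn by weight from DT_Enemies.
; It totals SpawnWeight across the table, then subtracts row weights from a random roll to pick each ID.
; The construction script sizes a box volume from extent variables.
; GetRandomLocationInVolume supplies spawn positions, though its random-point-in-box math appears unconnected.
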(event `self.ReceiveBeginPlay`
  (if (`self.Enabled`)
    (bind _returnvalue (`GameplayStatics.GetActorOfClass` null))
    (bind _totalweight (`self.CalculateTotalEnemyWeight`))
    (for _ (range 1 (+ (`self.NumItems`) 1))
      (bind _enemyid (`self.GetRandomEnemyToSpawn` _totalweight))
      (`|SpawnActorFromClass` "/Game/Blueprints/BP_Enemy.BP_Enemy_C" (`KismetMathLibrary.MakeTransform` (`self.GetRandomLocationInVolume`)) "AdjustIfPossibleButAlwaysSpawn" "OverrideRootScale" _returnvalue _enemyid null null))))

(fn `CalculateTotalEnemyWeight`
  (returns (TotalWeight :type "Float (double-precision)"))
  (locals (Weight :type "Float (double-precision)"))
  (bind _outrownames (`DataTableFunctionLibrary.GetDataTableRowNames` "/Game/Blueprints/DT_Enemies.DT_Enemies"))
  (for _array_element _outrownames
    (bind _returnvalue (`|GetDataTableRow` "/Game/Blueprints/DT_Enemies.DT_Enemies" _array_element)
      (:`then`
        (set `local.Weight` (+ (`local.Weight`) (`.SpawnWeight_14_F5E9F3E14F5B3008A156AA8D3002CEA8` (break `/Game/Blueprints/BP_EnemyStruct` _returnvalue)))))))
  (return (`local.Weight`)))

(fn `GetRandomEnemyToSpawn`
  (params (TotalPickupWeight :type "Float (double-precision)"))
  (returns (EnemyId :type Name))
  (locals (PickedRandom :type "Float (double-precision)") (FoundId :type Name))
  (set `local.PickedRandom` (`KismetMathLibrary.RandomFloatInRange` 0.0 (- TotalPickupWeight 1.0)))
  (bind _outrownames (`DataTableFunctionLibrary.GetDataTableRowNames` "/Game/Blueprints/DT_Enemies.DT_Enemies"))
  (for _array_element _outrownames
    (bind _returnvalue (`|GetDataTableRow` "/Game/Blueprints/DT_Enemies.DT_Enemies" _array_element)
      (:`then`
        (bind (_enemyid _displayname _flyspeed _damage _chaseradius _dieonpickuphit _staticmesh _spawnweight) (break `/Game/Blueprints/BP_EnemyStruct` _returnvalue))
        (bind _output_get (set `local.PickedRandom` (- (`local.PickedRandom`) _spawnweight)))
        (if (<= _output_get 0.0)
          (set `local.FoundId` _enemyid)
          (break)))))
  (return (`local.FoundId`)))

(fn `UserConstructionScript`
  (`BoxComponent.SetBoxExtent` (`self.Volume`) (`KismetMathLibrary.MakeVector` (`self.VolumeExtentsX`) (`self.VolumeExtentsY`) (`self.VolumeExtentsZ`)) true))