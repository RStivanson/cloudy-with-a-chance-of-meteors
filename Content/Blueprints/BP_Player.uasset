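; BP_Player is the player meteor pawn that flies toward BP_Earth, spinning on its roll axis as it moves.
; Axis inputs strafe the meteor, or rotate the Earth with roll zeroed while MoveEarth is held.
; A looping timer raises Heat, and pickups adjust both Heat and Size, with Size rescaling the meteor.
; It also creates the GameHUD on BeginPlay; RotateAroundEarth is defined but not called here.
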(event `Raise Heat`
  (`self.AdjustHeat` 1.0))

(event `self.ReceiveBeginPlay`
  ;[1 1 1] Get a reference to the Earth object
  (bind _returnvalue (`GameplayStatics.GetActorOfClass` "/Game/Blueprints/BP_Earth.BP_Earth_C"))
  (set `self.EarthObj` _returnvalue)
  (bind _returnvalue_2 (`|CreateWidget` "/Game/Blueprints/GameHUD.GameHUD_C" null self))
  (`UserWidget.AddToViewport` _returnvalue_2 0)
  (`KismetSystemLibrary.K2_SetTimerDelegate` (delegate `Raise Heat`) (`self.HeatRaiseTime`) true)
  (set `self.InitialMeteorScale` (`SceneComponent.RelativeScale3D` (`self.Scene`))))

(event `self.ReceiveTick`
  (params (DeltaSeconds :type "Float (single-precision)"))
  (bind (_x _y) (`KismetMathLibrary.BreakVector2D` (`self.MoveInput`)))
  (bind (_relativerotation_roll _relativerotation_pitch _relativerotation_yaw) (`KismetMathLibrary.BreakRotator` (`SceneComponent.RelativeRotation` (`self.Scene`))))
  ;[1 1 1] Rotate the meteor around its forward vector
  (`SceneComponent.K2_SetRelativeRotation` (`self.Scene`) (`KismetMathLibrary.MakeRotator` (+ (* DeltaSeconds (`self.RotateSpeed`)) _relativerotation_roll) _relativerotation_pitch _relativerotation_yaw) false false)
  ;[1 1 1] Move the meteor forward
  (`self.AddMovementInput` (+ (* (`self.GetForwardVectorToEarth`) (`self.FlySpeed`)) (* (`self.GetActorRightVector`) _x) (* (`self.GetActorUpVector`) _y))))

(event `InputAction|MoveEarth`
  (params (Key :type "Key Structure"))
  (:`Pressed`
    (set `self.IsMovingEarth` true))
  (:`Released`
    (set `self.IsMovingEarth` false)))

(event `/Game/Blueprints/BPI_Pickup.Pickup`
  (params (Pickup :type "/Game/Blueprints/BP_Pickup Object Reference"))
  (bind (_pickupdata_pickupid _pickupdata_displayname _pickupdata_sizemodifier _pickupdata_heatmodifier) (break `/Game/Blueprints/BP_PickupStruct` (`/Game/Blueprints/BP_Pickup.PickupData` Pickup)))
  (`self.AdjustSize` _pickupdata_sizemodifier)
  (`self.AdjustHeat` _pickupdata_heatmodifier))

(event `InputAxis|MoveHorizontal`
  (params (AxisValue :type "Float (single-precision)"))
  ;[1 1 1] Earth Movement
  (if (`self.IsMovingEarth`)
    (`self.RotateEarth` (`KismetMathLibrary.Vector_Up`) (* (`GameplayStatics.GetWorldDeltaSeconds`) (`self.EarthRotateSpeed`) AxisValue))
    (else
      (set `self.MoveInput` (`KismetMathLibrary.MakeVector2D` (* AxisValue (`self.StrafeSpeed`) -1.0) (`.Y` (`KismetMathLibrary.BreakVector2D` (`self.MoveInput`))))))))

(event `InputAxis|MoveVertical`
  (params (AxisValue :type "Float (single-precision)"))
  ;[1 1 1] Earth Movement
  (if (`self.IsMovingEarth`)
    (`self.RotateEarth` (`self.GetActorRightVector`) (* (`GameplayStatics.GetWorldDeltaSeconds`) (`self.EarthRotateSpeed`) AxisValue))
    (else
      (set `self.MoveInput` (`KismetMathLibrary.MakeVector2D` (`KismetMathLibrary.BreakVector2D` (`self.MoveInput`)) (* AxisValue (`self.StrafeSpeed`)))))))

(fn `AdjustHeat`
  (params (Adjustment :type "Float (double-precision)"))
  (set `self.Heat` (+ (`self.Heat`) Adjustment)))

(fn `AdjustSize`
  (params (Adjustment :type "Float (double-precision)"))
  (bind _output_get (set `self.Size` (+ (`self.Size`) Adjustment)))
  (`SceneComponent.SetRelativeScale3D` (`self.Scene`) (* (`self.InitialMeteorScale`) (+ (/ _output_get 10.0) 1.0))))

(fn `RotateAroundEarth`
  (params (Axis :type "Vector Structure") (Scale :type "Float (double-precision)"))
  (locals (Delta :type "Float (double-precision)"))
  (`self.K2_SetActorLocationAndRotation` (+ (`self.K2_GetActorLocation` (`self.EarthObj`)) (`KismetMathLibrary.RotateAngleAxis` (- (`self.K2_GetActorLocation`) (`self.K2_GetActorLocation` (`self.EarthObj`))) Scale Axis)) (`KismetMathLibrary.FindLookAtRotation` (`self.K2_GetActorLocation`) (`self.K2_GetActorLocation` (`self.EarthObj`)))))

(fn `RotateEarth`
  (params (Axis :type "Vector Structure") (Scale :type "Float (double-precision)"))
  (locals (Delta :type "Float (double-precision)"))
  (bind _earthobj (`self.EarthObj`))
  (bind _rootcomponent (`Actor.RootComponent` _earthobj))
  (bind (_returnvalue_roll _returnvalue_pitch _returnvalue_yaw) (`KismetMathLibrary.BreakRotator` (`SceneComponent.K2_GetComponentRotation` _rootcomponent)))
  ;[1 1 1] Rotate the earth object
  (`self.K2_AddActorWorldRotation` _earthobj (`KismetMathLibrary.RotatorFromAxisAndAngle` Axis Scale) false false)
  ;[1 1 1] Contrain the X rotation axis to prevent odd rotations
  (`SceneComponent.K2_SetWorldRotation` _rootcomponent (`KismetMathLibrary.MakeRotator` 0.0 _returnvalue_pitch _returnvalue_yaw) false false))

(fn `UserConstructionScript`)